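; Terrain tile for an infinite-terrain mode that scatters random numbers of containers, canisters, boxes, barriers and rocks via PlaceActors on BeginPlay.
; The player entering LockingBox turns the barrier green and passable; leaving turns it red and solid, then asks InfiniteTerrain_GM to spawn a tile.
; The player overlapping DestroyBox destroys the tile.
; GetAttachedLocation exposes the Arrow's world transform as an attachment point.
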(event `self.ReceiveBeginPlay`
  (`self.PlaceActors` "/Game/Dynamic/Terrain/Props/Container_BP.Container_BP_C" 1 5)
  (`self.PlaceActors` "/Game/Dynamic/Terrain/Props/Canister_BP.Canister_BP_C" 1 2)
  (`self.PlaceActors` "/Game/Dynamic/Terrain/Props/Box_BP.Box_BP_C" 0 4)
  (`self.PlaceActors` "/Game/Dynamic/Terrain/Props/Barrier_BP.Barrier_BP_C" 0 2)
  (`self.PlaceActors` "/Game/Dynamic/Terrain/Props/Box_BP.Box_BP_C" 0 4)
  (`self.PlaceActors` "/Game/Dynamic/Terrain/Props/Rock01_BP.Rock01_BP_C" 0 3)
  (`self.PlaceActors` "/Game/Dynamic/Terrain/Props/Rock05_BP.Rock05_BP_C" 0 3)
  (`self.PlaceActors` "/Game/Dynamic/Terrain/Props/Rock17_BP.Rock17_BP_C" 0 3))

(event `self.LockingBox.OnComponentBeginOverlap`
  (params (OverlappedComponent :type "PrimitiveComponent Object Reference") (OtherActor :type "Actor Object Reference") (OtherComp :type "PrimitiveComponent Object Reference") (OtherBodyIndex :type Integer) (bFromSweep :type Boolean) (SweepResult :type "HitResult Structure (by ref)"))
  (`self.IsPlayer` OtherActor)
  (`self.Unlock`))

(event `self.LockingBox.OnComponentEndOverlap`
  (params (OverlappedComponent :type "PrimitiveComponent Object Reference") (OtherActor :type "Actor Object Reference") (OtherComp :type "PrimitiveComponent Object Reference") (OtherBodyIndex :type Integer))
  (`self.IsPlayer` OtherActor)
  (`self.Lock`)
  (bind _asinfinite_terrain_gm (cast `/Game/Dynamic/GameMode/InfiniteTerrain_GM` (`GameplayStatics.GetGameMode`)))
  (`/Game/Dynamic/GameMode/InfiniteTerrain_GM.SpawnTile` _asinfinite_terrain_gm))

(event `self.DestroyBox.OnComponentBeginOverlap`
  (params (OverlappedComponent :type "PrimitiveComponent Object Reference") (OtherActor :type "Actor Object Reference") (OtherComp :type "PrimitiveComponent Object Reference") (OtherBodyIndex :type Integer) (bFromSweep :type Boolean) (SweepResult :type "HitResult Structure (by ref)"))
  (`self.IsPlayer` OtherActor)
  (`self.K2_DestroyActor`))

(fn `GetAttachedLocation`
  (returns (AttachTransform :type "Transform Structure"))
  (return (`SceneComponent.K2_GetComponentToWorld` (`self.Arrow`))))

(fn `Lock`
  (bind _barrier (`self.Barrier`))
  (`PrimitiveComponent.SetMaterial` _barrier 0 "/Game/Dynamic/Terrain/Material/Red_BarrierMaterial.Red_BarrierMaterial")
  (`PrimitiveComponent.SetCollisionEnabled` _barrier "QueryAndPhysics"))

(fn `Unlock`
  (bind _barrier (`self.Barrier`))
  (`PrimitiveComponent.SetMaterial` _barrier 0 "/Game/Dynamic/Terrain/Material/Green_BarrierMaterial.Green_BarrierMaterial")
  (`PrimitiveComponent.SetCollisionEnabled` _barrier "NoCollision"))

(fn `UserConstructionScript`)